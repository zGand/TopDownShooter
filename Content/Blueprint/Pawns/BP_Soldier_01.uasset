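; Player soldier pawn for what appears to be a top-down shooter, with world-axis movement, rifle fire and a HUD widget.
; Each tick, mouse movement direction above a deadzone smoothly turns the control rotation to aim.
; Pressing fire starts muzzle flash and sound until release, but runs only one damaging line trace from the muzzle socket.
; Damage lowers clamped health; at zero the soldier is flagged dead, blocking movement and aiming.
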(event `self.ReceiveBeginPlay`
  (bind _returnvalue (`|CreateWidget` "/Game/UI/W_PlayerHUD.W_PlayerHUD_C" null self))
  (`UserWidget.AddToViewport` _returnvalue 0))

(event `self.ReceiveTick`
  (params (DeltaSeconds :type "Float (single-precision)"))
  (`self.UpdatePlayerAim`))

(event `InputAxis|MovingForwardBackward`
  (params (AxisValue :type "Float (single-precision)"))
  (if (`self.IsAlive`)
    (`self.AddMovementInput` (1.0 0.0 0.0) AxisValue)))

(event `InputAxis|MovingLeftRight`
  (params (AxisValue :type "Float (single-precision)"))
  (if (`self.IsAlive`)
    (`self.AddMovementInput` (0.0 1.0 0.0) AxisValue)))

(event `InputAction|FireWeapon`
  (params (Key :type "Key Structure"))
  (:`Pressed`
    (`self.StartFireWeapon`)
    (`self.WeaponTrace`))
  (:`Released`
    (`self.StopFireWeapon`)))

(event `self.ReceiveAnyDamage`
  (params (Damage :type "Float (single-precision)") (DamageType :type "DamageType Object Reference") (InstigatedBy :type "Controller Object Reference") (DamageCauser :type "Actor Object Reference"))
  (bind _health (`self.DecreaseHealth` Damage))
  (if (== _health 0.0)
    (set `self.Dead` true)
    (`self.StopFireWeapon`)))

(fn `DecreaseHealth`
  (params (DamageAmount :type "Float (double-precision)"))
  (returns (Health :type "Float (double-precision)"))
  (bind _output_get (set `self.Health` (`KismetMathLibrary.FClamp` (- (`self.Health`) DamageAmount) 0.0 100.0)))
  (return _output_get))

(fn `GetMouseVelocity`
  (returns (ReturnValue :type "Vector2D Structure"))
  (bind (_deltax _deltay) (`PlayerController.GetInputMouseDelta` (`GameplayStatics.GetPlayerController` 0)))
  (return (/ (`KismetMathLibrary.MakeVector2D` _deltax _deltay) (`GameplayStatics.GetWorldDeltaSeconds`))))

(fn `GetWeaponTraceEndLocation`
  (returns (ReturnValue :type "Vector Structure"))
  (return (+ (`self.GetWeaponTraceStartLocation`) (* (`KismetMathLibrary.GetForwardVector` (`self.GetControlRotation`)) (`self.WeaponRange`)))))

(fn `GetWeaponTraceStartLocation`
  (returns (ReturnValue :type "Vector Structure"))
  (return (`SceneComponent.GetSocketLocation` (`self.Rifle`) "MuzzleFlashSocket")))

(fn `IsAlive`
  (returns (ReturnValue :type Boolean))
  (return (not (`self.Dead`))))

(fn `IsMouseAboveDeadzone`
  (returns (ReturnValue :type Boolean))
  (return (> (`KismetMathLibrary.VSize2D` (`self.GetMouseVelocity`)) (`self.MouseDeadzone`))))

(fn `StartFireWeapon`
  (if (`self.IsAlive`)
    (`ActorComponent.Activate` (`self.P_AssaultRifle_MF`) false)
    (bind _returnvalue (`GameplayStatics.SpawnSound2D` "/Game/Sounds/Weapon_AssaultRifle/Stereo/RifleSouindCue.RifleSouindCue" 1.0 1.0 0.0 null))
    (set `self.WeaponFireSound` _returnvalue)))

(fn `StopFireWeapon`
  (`ActorComponent.Deactivate` (`self.P_AssaultRifle_MF`))
  (`AudioComponent.Stop` (`self.WeaponFireSound`))
  (if (`self.IsAlive`)
    (`GameplayStatics.SpawnSound2D` "/Game/Sounds/Weapon_AssaultRifle/Stereo/RifleFireEnd.RifleFireEnd" 1.0 1.0 0.0 null)))

(fn `UpdatePlayerAim`
  (bind _returnvalue (`GameplayStatics.GetPlayerController` 0))
  (bind (_returnvalue_x _returnvalue_y) (`KismetMathLibrary.BreakVector2D` (`self.GetMouseVelocity`)))
  (if (`self.IsAlive`)
    (if (`self.IsMouseAboveDeadzone`)
      (`Controller.SetControlRotation` _returnvalue (`KismetMathLibrary.RInterpTo` (`Controller.GetControlRotation` _returnvalue) (`KismetMathLibrary.MakeRotator` 0.0 0.0 (`KismetMathLibrary.DegAtan2` _returnvalue_x _returnvalue_y)) (`GameplayStatics.GetWorldDeltaSeconds`) (`self.MouseSmoothingStrength`))))))

(fn `UserConstructionScript`)

(fn `WeaponTrace`
  (bind _outhit (`KismetSystemLibrary.LineTraceSingle` (`self.GetWeaponTraceStartLocation`) (`self.GetWeaponTraceEndLocation`) "TraceTypeQuery1"))
  (bind (_bblockinghit _binitialoverlap _time _distance _location _impactpoint _normal _impactnormal _physmat _hitactor) (`GameplayStatics.BreakHitResult` _outhit))
  (if _bblockinghit
    (`GameplayStatics.ApplyDamage` _hitactor (`self.DamagePerShot`))))